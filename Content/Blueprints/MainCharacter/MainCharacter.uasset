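; Main character pawn that stands idle until the puzzle is solved, then starts walking.
; Tick reads IsThePuzzleSolved, set through the IsPuzzleSolved function, to toggle visibility between the Idle and Move components.
; While solved, it feeds CharacterLocation to AddMovementInput as the direction; the node that sets that variable is unconnected.
; BeginPlay locks the Y axis and disables physics simulation.
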(event EventTick
  (params (DeltaSeconds :type Float%20%28single-precision%29))
  (if (Variables|Default|GetIsThePuzzleSolved?)
    (Rendering|SetVisibility (Variables|Default|GetIdle) false false)
    (Rendering|SetVisibility (Variables|Default|GetMove) true false)
    (Pawn|Input|AddMovementInput (Variables|Default|GetCharacterLocation) 1.0 false)
    (else
      (Rendering|SetVisibility (Variables|Default|GetMove) false false)
      (Rendering|SetVisibility (Variables|Default|GetIdle) true false))))

(event EventBeginPlay
  (Class|PrimitiveComponent|SetLockedAxis "Y")
  (Physics|SetSimulatePhysics false))

(fn ConstructionScript)

(fn IsPuzzleSolved?
  (params (IsThePuzzleSolved? :type Boolean))
  (Variables|Default|SetIsThePuzzleSolved? IsThePuzzleSolved?))