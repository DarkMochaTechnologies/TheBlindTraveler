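; Breakable telephone pole puzzle actor that reacts to an Axe overlapping its collision while the Ok flag is true.
; The overlap destroys the actor after a short delay.
; Tick tests the same overlapped actor and flag, removes the intact pole component once and toggles the broken-pole component visible, then hidden after a brief delay.
; IsAxe only stores a Pixaxe flag, whose destroy check is unconnected.
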(event OnComponentBeginOverlap(Collicion)
  (params (OtherActor :type Actor%20Object%20Reference) (OtherComp :type Primitive%20Component%20Object%20Reference) (OtherBodyIndex :type Integer) (bFromSweep :type Boolean) (SweepResult :type Hit%20Result%20Structure%20%28by%20ref%29))
  (if (and (== (Utilities|GetClass OtherActor) "/Game/Blueprints/Tools/Axe.Axe_C") (Variables|Default|GetOk?))
    (Utilities|FlowControl|Delay 1.5)
    (Actor|DestroyActor)))

(event EventTick
  (params (DeltaSeconds :type Float%20%28single-precision%29))
  (if (and (== (Utilities|GetClass (stale OnComponentBeginOverlap(Collicion) OtherActor)) "/Game/Blueprints/Tools/Axe.Axe_C") (Variables|Default|GetOk?))
    (Utilities|FlowControl|Sequence
      (:then_0
        (Utilities|FlowControl|DoOnce false
          (:Completed
            (Components|DestroyComponent (Variables|Default|GetT_Pole)))))
      (:then_1
        (Rendering|SetVisibility (Variables|Default|GetT_PoleBreak) true false)
        (Utilities|FlowControl|Delay 0.2)
        (Rendering|SetVisibility (Variables|Default|GetT_PoleBreak) false false)))))

(fn ConstructionScript)

(fn IsAxe
  (params (Axe :type Boolean))
  (Variables|Default|Setpixaxe Axe))