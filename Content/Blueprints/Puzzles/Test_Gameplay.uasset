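; Test gameplay Blueprint that lets the player grab and carry light physics objects with the left mouse button.
; On press, a one-unit camera-forward trace finds a physics body or pawn under a mass limit and grabs it with a newly added PhysicsHandle.
; Tick pulls the handle target to the actor's own location until release.
; The PickupDistance scaling and hit-offset math are left unconnected.
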(event EventTick
  (params (DeltaSeconds :type Float%20%28single-precision%29))
  (if (Variables|Default|GetPhysicsHandleActive)
    (Variables|Default|SetHandleLocation (Transformation|GetActorLocation))
    (Physics|Components|PhysicsHandle|SetTargetLocation (Variables|Default|GetPhysicsHandle) (Variables|Default|GetHandleLocation))))

(event Input|MouseEvents|LeftMouseButton
  (bind _camera (Variables|Default|GetCamera))
  (bind _returnvalue (Transformation|GetWorldLocation _camera))
  (:Pressed
    (Variables|Default|SetPhysicsHandleActive true)
    (bind (_outhit _returnvalue_2) (Collision|LineTraceForObjects _returnvalue (+ _returnvalue (Math|Vector|GetForwardVector _camera)) (Utilities|Array|MakeArray "ObjectTypeQuery4" "ObjectTypeQuery3") false 0 "None"))
    (Variables|Default|SetOtherItemLocation "0, 0, 0")
    (if _returnvalue_2
      (if (< (Physics|GetMass (.HitComponent (Collision|BreakHitResult _outhit))) 5e+02)
        (bind _returnvalue_3 (AddComponent|AddPhysicsHandleComponent false (Transformation|GetActorTransform)))
        (Variables|Default|SetPhysicsHandle _returnvalue_3)
        (Variables|Default|SetPhysicsObject (.HitComponent (Collision|BreakHitResult _outhit)))
        (Class|PhysicsHandleComponent|GrabComponent (Variables|Default|GetPhysicsHandle) (.HitComponent (Collision|BreakHitResult _outhit)) (.HitBoneName (Collision|BreakHitResult _outhit)) "0, 0, 0" false))))
  (:Released
    (Variables|Default|SetPhysicsHandleActive false)
    (Physics|Components|PhysicsHandle|ReleaseComponent (Variables|Default|GetPhysicsHandle))))

(fn ConstructionScript)