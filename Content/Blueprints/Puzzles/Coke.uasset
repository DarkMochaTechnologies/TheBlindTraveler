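; Puzzle actor for a Coke item that is disposed of when it touches a TrashCan, with movement locked on the Y axis from BeginPlay.
; On that overlap it destroys its trigger collision, disables the Coke's collision, reveals Hand1 and moves the Coke just below that hand.
; The actor destroys itself after a short delay.
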(event OnComponentBeginOverlap(cokeCollision)
  (params (OtherActor :type Actor%20Object%20Reference) (OtherComp :type Primitive%20Component%20Object%20Reference) (OtherBodyIndex :type Integer) (bFromSweep :type Boolean) (SweepResult :type Hit%20Result%20Structure%20%28by%20ref%29))
  (if (== (Utilities|GetClass OtherActor) "/Game/Blueprints/Tools/TrashCan.TrashCan_C")
    (Components|DestroyComponent (Variables|Default|GetcokeCollision))
    (Collision|SetCollisionEnabled (Variables|Default|Getcoke) "NoCollision")
    (Rendering|SetVisibility (Variables|Default|GetHand-1) true false)
    (Transformation|SetWorldLocation (Variables|Default|Getcoke) (+ (Transformation|GetWorldLocation (Variables|Default|GetHand-1)) "0, 0,-5.000000") false)
    (Utilities|FlowControl|Delay 2.0)
    (Actor|DestroyActor)))

(event EventBeginPlay
  (Class|PrimitiveComponent|SetLockedAxis "Y"))

(fn ConstructionScript)