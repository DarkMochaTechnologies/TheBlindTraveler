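; FireGround is a 2D puzzle Blueprint with box and flipbook components that are removed by mouse interaction.
; Clicking the box destroys it, while the flipbook is destroyed on cursor hover, or on click after a debug "Hello" print.
; BeginPlay locks the Y axis, and left mouse calls Possess on the player controller with no pawn supplied.
; An actor-destroy branch is left unconnected and never runs.
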(event OnClicked(Box1)
  (params (TouchedComponent :type Primitive%20Component%20Object%20Reference))
  (Components|DestroyComponent TouchedComponent))

(event OnBeginCursorOver(PaperFlipbook1)
  (params (TouchedComponent :type Primitive%20Component%20Object%20Reference))
  (Components|DestroyComponent TouchedComponent))

(event OnClicked(PaperFlipbook1)
  (params (TouchedComponent :type Primitive%20Component%20Object%20Reference))
  (Development|PrintString "Hello")
  (Components|DestroyComponent (stale OnBeginCursorOver(PaperFlipbook1) TouchedComponent)))

(event EventBeginPlay
  (Class|PrimitiveComponent|SetLockedAxis "Y")
  (Class|PrimitiveComponent|SetLockedAxis "Y"))

(event Input|MouseEvents|LeftMouseButton
  (:Pressed
    (Pawn|Possess (Game|GetPlayerController 0))))

(fn ConstructionScript)