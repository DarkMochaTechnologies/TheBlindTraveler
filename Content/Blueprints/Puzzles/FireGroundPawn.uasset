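; FireGroundPawn is a puzzle pawn for a ground fire that is removed when its box is overlapped while the bucket condition is set.
; It locks movement on the Y axis at BeginPlay.
; IsBucket stores the Bucket flag from outside, and a Box1 overlap checks only that flag, not the overlapping actor.
; On success it destroys itself, then sets Collided, which GetCollided exposes.
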(event OnComponentBeginOverlap(Box1)
  (params (OtherActor :type Actor%20Object%20Reference) (OtherComp :type Primitive%20Component%20Object%20Reference) (OtherBodyIndex :type Integer) (bFromSweep :type Boolean) (SweepResult :type Hit%20Result%20Structure%20%28by%20ref%29))
  (if (Variables|Default|GetBucket)
    (Actor|DestroyActor)
    (Variables|Default|SetCollided? true)))

(event EventBeginPlay
  (Class|PrimitiveComponent|SetLockedAxis "Y"))

(fn ConstructionScript)

(fn IsBucket
  (params (Bucket :type Boolean))
  (Variables|Default|SetBucket Bucket))

(fn GetCollided
  (return (Variables|Default|GetCollided?)))