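; LighterTool is a lighter tool that switches between lit and unlit visuals.
; TriggerLighter takes a boolean and toggles component visibility, with false hiding Fire and LighterLit and showing the plain Lighter.
; LighterLocation returns the first player controller's mouse position as a 2D vector, though nothing in this file applies it to the lighter.
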(fn ConstructionScript)

(fn TriggerLighter
  (params (Trigger :type Boolean))
  (if Trigger
    (Rendering|SetVisibility true false)
    (Rendering|SetVisibility true false)
    (Rendering|SetVisibility false false)
    (else
      (Rendering|SetVisibility (Variables|Default|GetFire) false false)
      (Rendering|SetVisibility (Variables|Default|GetLighterLit) false false)
      (Rendering|SetVisibility (Variables|Default|GetLighter) true false))))

(fn LighterLocation
  (bind _returnvalue (Game|GetPlayerController 0))
  (bind (_locationx _locationy) (Game|Player|GetMousePosition _returnvalue))
  (return (Math|Vector2D|MakeVector2D _locationx _locationy)))