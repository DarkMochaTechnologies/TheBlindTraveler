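; MyCharacter is a player character that moves along the world X axis and can pause the game.
; The MoveRight axis adds movement input and snaps the controller's yaw to face the direction of travel, as in a side-scroller.
; The Pause action toggles game pause, creating and showing a PauseMenu widget when pausing and removing it when resuming.
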(event Input|ActionEvents|InputActionPause
  ;[1 1 1] Handling Pause
  (:Pressed
    (if (Game|IsGamePaused)
      (Game|SetGamePaused false)
      (Widget|RemovefromParent (Variables|Default|GetPauseMenu))
      (else
        (Game|SetGamePaused true)
        (bind _returnvalue (UserInterface|CreateWidget "/Game/Menus/PauseMenu.PauseMenu_C"))
        (Variables|Default|SetPauseMenu _returnvalue)
        (UserInterface|Viewport|AddtoViewport (Variables|Default|GetPauseMenu))))))

(event Input|AxisEvents|InputAxisMoveRight
  (params (AxisValue :type Float%20%28single-precision%29))
  ;[1 1 1] Handle movement
  (Pawn|Input|AddMovementInput "1.000000, 0,0.000000" AxisValue false)
  (Math|Float|CompareFloat AxisValue 0.0
    (:>
      (Pawn|SetControlRotation (Pawn|GetController) (Class|KismetMathLibrary|MakeRot 0.0 0.0 0.0)))
    (:<
      (Pawn|SetControlRotation (Pawn|GetController) (Class|KismetMathLibrary|MakeRot 0.0 1.8e+02 0.0)))))

(fn ConstructionScript)