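; CustomCursor is a HUD Blueprint that draws a custom mouse cursor texture on screen.
; Each DrawHUD call reads the first player controller's mouse position and draws a fixed-size square texture centered on it.
; The position is shifted by the difference between the HUD draw size and the controller's viewport size.
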(event EventDrawHUD
  (params (SizeX :type Integer) (SizeY :type Integer))
  (bind _returnvalue (Game|GetPlayerController 0))
  (bind _returnvalue_2 (Math|Float|MakeLiteralFloat 32.0))
  (bind (_locationx _locationy) (Game|Player|GetMousePosition _returnvalue))
  (bind (_sizex _sizey) (HUD|GetViewportSize _returnvalue))
  (bind _returnvalue_3 (/ _returnvalue_2 2.0))
  (Canvas|DrawTexture "/Game/Textures/Tools/LighterwithFire/1.1" (- (+ _locationx (Math|Conversions|ToFloat(Integer) (- SizeX _sizex))) _returnvalue_3) (- (+ (Math|Conversions|ToFloat(Integer) (- SizeY _sizey)) _locationy) _returnvalue_3) _returnvalue_2 _returnvalue_2 0.0 0.0 1.0 1.0 "(R=1.000000,G=1.000000,B=1.000000,A=1.000000)"))

(fn ConstructionScript)