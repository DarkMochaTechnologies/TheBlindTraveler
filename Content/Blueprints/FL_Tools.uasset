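; Blueprint function library of shared helpers for spawning, audio volume and save games in a puzzle game.
; Spawn functions place puzzles randomly in the XZ plane at Y=0, or create tools and cursors at the deprojected mouse position, replacing the current sprite.
; Volume helpers multiply saved master and channel settings, with fallbacks when no save exists.
; Progress helpers check, read and write level, checkpoint and unlocked-level saves using ConstantNames slot names.
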(fn CreatePuzzles
  (params (Class :type Pawn%20Class%20Reference) (TransformMin :type Transform) (TransformMax :type Transform))
  (bind _location (Math|Transform|BreakTransform TransformMin))
  (bind _location_2 (Math|Transform|BreakTransform TransformMax))
  (bind (_x _y _z) (Math|Vector|BreakVector _location_2))
  (bind (_x_2 _y_2 _z_2) (Math|Vector|BreakVector _location))
  (bind _returnvalue (Game|SpawnActorfromClass Class (Math|Conversions|ToTransform(Vector) (Math|Vector|MakeVector (Math|Random|RandomFloatinRange _x_2 _x) 0.0 (Math|Random|RandomFloatinRange _z_2 _z))) false 0))
  (return _returnvalue))

(fn SpawnTools
  (params (Tool%20Class :type Actor%20Class%20Reference) (Current%20Sprite :type Actor%20Object%20Reference))
  (bind _returnvalue (Game|GetPlayerController 0))
  (bind _worldlocation (Game|Player|ConvertMouseLocationToWorldSpace _returnvalue))
  (bind (_x _y _z) (Math|Vector|BreakVector _worldlocation))
  (bind _returnvalue_2 (Game|SpawnActorfromClass Tool%20Class (Math|Conversions|ToTransform(Vector) (Math|Vector|MakeVector _x 0.0 _z)) false 0))
  (Actor|DestroyActor Current%20Sprite)
  (return _returnvalue_2))

(fn UseGameCursor
  (params (Current%20Sprite :type Actor%20Object%20Reference))
  (bind _returnvalue (Game|SpawnActorfromClass "/Game/Blueprints/Misc/Cursor.Cursor_C" (Math|Conversions|ToTransform(Vector) (.WorldLocation (Game|Player|ConvertMouseLocationToWorldSpace (Game|GetPlayerController 0)))) false 0))
  (if (Utilities|IsValid Current%20Sprite)
    (Actor|DestroyActor Current%20Sprite))
  (return _returnvalue))

(fn SetComponentMusicVolume
  (params (MusicComponent :type Audio%20Component%20Object%20Reference) (ConstantNames :type Constant%20Names%20Structure))
  (bind _savesettingsfilename (Utilities|Struct|BreakConstantNames ConstantNames))
  (LocalVariables|SetAudio MusicComponent)
  (bind _returnvalue (SaveGame|DoesSaveGameExist _savesettingsfilename))
  (if _returnvalue
    (bind _returnvalue_2 (SaveGame|LoadGamefromSlot _savesettingsfilename))
    (bind _assave_settings (Utilities|Casting|CastToSaveSettings _returnvalue_2))
    (LocalVariables|SetMusicMultiplier (* (/ (Math|Conversions|ToFloat(Integer) (Variables|/Game/Save/SaveSettings.SaveSettings_C|GetMasterVolume _assave_settings)) 1e+01) (/ (Math|Conversions|ToFloat(Integer) (Variables|/Game/Save/SaveSettings.SaveSettings_C|GetMusicVolume _assave_settings)) 1e+01)))
    (else
      (LocalVariables|SetMusicMultiplier 0.5)))
  (Audio|Components|Audio|SetVolumeMultiplier (LocalVariables|GetAudio) (LocalVariables|GetMusicMultiplier) :!class /Script/Engine.AudioComponent))

(fn SetComponentSFXVolume
  (params (SFXComponent :type Audio%20Component%20Object%20Reference) (ConstantNames :type Constant%20Names%20Structure))
  (bind _savesettingsfilename (Utilities|Struct|BreakConstantNames ConstantNames))
  (LocalVariables|SetAudio SFXComponent)
  (bind _returnvalue (SaveGame|DoesSaveGameExist _savesettingsfilename))
  (if _returnvalue
    (bind _returnvalue_2 (SaveGame|LoadGamefromSlot _savesettingsfilename))
    (bind _assave_settings (Utilities|Casting|CastToSaveSettings _returnvalue_2))
    (LocalVariables|SetSFXMultiplier (* (/ (Math|Conversions|ToFloat(Integer) (Variables|/Game/Save/SaveSettings.SaveSettings_C|GetMasterVolume _assave_settings)) 1e+01) (/ (Math|Conversions|ToFloat(Integer) (Variables|/Game/Save/SaveSettings.SaveSettings_C|GetSoundEffectsVolume _assave_settings)) 1e+01)))
    (else
      (LocalVariables|SetSFXMultiplier (* 0.5 0.5))))
  (Audio|Components|Audio|SetVolumeMultiplier (LocalVariables|GetAudio) (LocalVariables|GetSFXMultiplier) :!class /Script/Engine.AudioComponent))

(fn GetMusicVolume
  (params (ConstantNames :type Constant%20Names%20Structure))
  (bind _savesettingsfilename (Utilities|Struct|BreakConstantNames ConstantNames))
  (bind _returnvalue (SaveGame|DoesSaveGameExist _savesettingsfilename))
  (if _returnvalue
    (bind _returnvalue_2 (SaveGame|LoadGamefromSlot _savesettingsfilename))
    (bind _assave_settings (Utilities|Casting|CastToSaveSettings _returnvalue_2))
    (LocalVariables|SetMusicVolumeMultiplier (* (/ (Math|Conversions|ToFloat(Integer) (Variables|/Game/Save/SaveSettings.SaveSettings_C|GetMasterVolume _assave_settings)) 1e+01) (/ (Math|Conversions|ToFloat(Integer) (Variables|/Game/Save/SaveSettings.SaveSettings_C|GetMusicVolume _assave_settings)) 1e+01)))
    (else
      (LocalVariables|SetMusicVolumeMultiplier 0.5)))
  (return (LocalVariables|GetMusicVolumeMultiplier)))

(fn GetLevelNameandCheckpoint
  (params (ConstantNames :type Constant%20Names%20Structure))
  (bind (_gamesavefilename _levelnames) (Utilities|Struct|BreakConstantNames ConstantNames))
  (LocalVariables|SetFileName _gamesavefilename)
  (LocalVariables|SetLevelNames _levelnames)
  (bind _returnvalue (SaveGame|LoadGamefromSlot (LocalVariables|GetFileName)))
  (bind _asgame_save (Utilities|Casting|CastToGameSave _returnvalue))
  (return (Utilities|Array|Get(acopy) (LocalVariables|GetLevelNames) (- (Variables|/Game/Save/GameSave.GameSave_C|GetLevelProgress _asgame_save) 1)) (Variables|/Game/Save/GameSave.GameSave_C|GetCheckpointProgress _asgame_save)))

(fn CheckGameSaveExist
  (params (ConstantNames :type Constant%20Names%20Structure))
  (bind _returnvalue (SaveGame|DoesSaveGameExist (.GameSaveFileName (Utilities|Struct|BreakConstantNames ConstantNames))))
  (return _returnvalue))

(fn UpdateUnlockedLevels
  (params (UpdatedLevels :type Array%20of%20Booleans) (SaveGameObject :type Save%20Game%20Object%20Reference))
  (bind _assave_unlocked_levels (Utilities|Casting|CastToSaveUnlockedLevels SaveGameObject))
  (Variables|/Game/Save/SaveUnlockedLevels.SaveUnlockedLevels_C|SetLevels _assave_unlocked_levels UpdatedLevels)
  (SaveGame|SaveGametoSlot _assave_unlocked_levels (.UnlockedLevelsFileName (Utilities|Struct|BreakConstantNames (LocalVariables|GetConstantNames)))))

(fn UpdateGameSave
  (params (LevelProgress :type Integer) (CheckpointProgess :type Integer) (SaveGame :type Save%20Game%20Object%20Reference))
  (bind _asgame_save (Utilities|Casting|CastToGameSave SaveGame))
  (Variables|/Game/Save/GameSave.GameSave_C|SetCheckpointProgress _asgame_save CheckpointProgess)
  (Variables|/Game/Save/GameSave.GameSave_C|SetLevelProgress _asgame_save LevelProgress)
  (SaveGame|SaveGametoSlot _asgame_save (.GameSaveFileName (Utilities|Struct|BreakConstantNames (LocalVariables|GetConstantNames)))))